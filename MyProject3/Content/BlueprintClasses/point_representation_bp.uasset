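; Actor Blueprint that represents a numbered point in the world as a colored static mesh placed at a stored coordinate.
; The construction script derives a color from Id with modulo math, sets it as the mesh materials' "Color" parameter, and prints the three components as debug output.
; BeginPlay prints the Id, and Tick moves the actor to Coords every frame without sweeping.
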(event `self.ReceiveBeginPlay`
  (`KismetSystemLibrary.PrintText` (`KismetTextLibrary.Conv_IntToText` (`self.id`))))

(event `self.ReceiveTick`
  (params (DeltaSeconds :type "Float (single-precision)"))
  (`self.K2_SetActorLocation` (`self.coords`)))

(fn `UserConstructionScript`
  (bind _returnvalue (* (`KismetMathLibrary.Conv_IntToDouble` (mod (`self.id`) 6)) 0.2))
  (bind _returnvalue_2 (* (`KismetMathLibrary.Conv_IntToDouble` (mod (`self.id`) 8)) 0.14))
  (bind _returnvalue_3 (* (`KismetMathLibrary.Conv_IntToDouble` (mod (`self.id`) 3)) 0.5))
  (`MeshComponent.SetVectorParameterValueOnMaterials` (`self.StaticMesh`) "Color" (`KismetMathLibrary.MakeVector` _returnvalue_2 _returnvalue_3 _returnvalue))
  (`KismetSystemLibrary.PrintText` (`KismetTextLibrary.Conv_DoubleToText` _returnvalue_2 "HalfToEven"))
  (`KismetSystemLibrary.PrintText` (`KismetTextLibrary.Conv_DoubleToText` _returnvalue_3 "HalfToEven"))
  (`KismetSystemLibrary.PrintText` (`KismetTextLibrary.Conv_DoubleToText` _returnvalue "HalfToEven")))